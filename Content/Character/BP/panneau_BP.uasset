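; Interactable sign Blueprint (panneau) that shows its text on screen when interacted with.
; The Interact event acts as a toggle: if a dialogue widget is valid, it removes it and clears the reference.
; Otherwise it creates a BP_inter widget for the first player controller, adds it to the viewport and sets its DialogueText from MyText.
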(event EventInteract
  (Utilities|IsValid (Variables|Default|Getdialogue%20widget)
    (:Is%20Valid
      (Widget|RemovefromParent (Variables|Default|Getdialogue%20widget))
      (Variables|Default|Setdialogue%20widget 0))
    (:Is%20Not%20Valid
      (bind _returnvalue (UserInterface|CreateWidget "/Game/Character/BP/BP_inter.BP_inter_C" (Game|GetPlayerController 0)))
      (bind _output_get (Variables|Default|Setdialogue%20widget _returnvalue))
      (UserInterface|Viewport|AddtoViewport _output_get 0)
      (Variables|/Game/Character/BP/BP_inter.BP_inter_C|SetDialogueText (Variables|Default|Getdialogue%20widget) (Variables|Default|GetMyText)))))

(fn ConstructionScript)